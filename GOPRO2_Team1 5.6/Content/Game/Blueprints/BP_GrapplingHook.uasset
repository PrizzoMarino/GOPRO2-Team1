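; BP_GrapplingHook is a projectile grappling hook that latches onto whatever its sphere overlaps.
; On overlap it stops its projectile movement, records the hit location and marks itself hooked.
; It switches the owning BP_CharacterTest to Flying, flags the grapple hit, deducts one energy clamped at zero and refreshes the HUD.
; Tick is empty, so no pull movement happens in this Blueprint.
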(event OnComponentBeginOverlap(Sphere)
  (params (OverlappedComponent :type Primitive%20Component%20Object%20Reference) (OtherActor :type Actor%20Object%20Reference) (OtherComp :type Primitive%20Component%20Object%20Reference) (OtherBodyIndex :type Integer) (bFromSweep :type Boolean) (SweepResult :type Hit%20Result%20Structure%20%28by%20ref%29))
  (bind _returnvalue (Transformation|GetActorLocation))
  (Components|Movement|StopMovementImmediately (Variables|Default|GetProjectileMovement))
  (bind _asbp_character_test (Utilities|Casting|CastToBP_CharacterTest (Components|GetOwner)))
  (Pawn|Components|CharacterMovement|SetMovementMode (Variables|/Script/Engine.Character|GetCharacterMovement _asbp_character_test) "MOVE_Flying" 0)
  (Variables|Default|SetHookLocation (Math|Vector|MakeVector (.x _returnvalue) (.y _returnvalue) (.z _returnvalue)))
  (Transformation|AttachComponentToComponent OverlappedComponent "None" "KeepWorld" "KeepWorld" "KeepRelative" true)
  (Variables|Default|SetbIsHooked true)
  (Variables|/Game/Test/BP_CharacterTest.BP_CharacterTest_C|SetbGrappleHitSurface _asbp_character_test true)
  (bind _output_get (Variables|/Game/Test/BP_CharacterTest.BP_CharacterTest_C|SetCurrentEnergy _asbp_character_test (Math|Integer|Max(Integer) 0 (- (Variables|/Game/Test/BP_CharacterTest.BP_CharacterTest_C|GetCurrentEnergy _asbp_character_test) 1))))
  (Utilities|IsValid (Variables|/Game/Test/BP_CharacterTest.BP_CharacterTest_C|GetWBP_HUD _asbp_character_test)
    (:Is%20Valid
      (Default|SetEnergy (Variables|/Game/Test/BP_CharacterTest.BP_CharacterTest_C|GetWBP_HUD _asbp_character_test) _output_get (Variables|/Game/Test/BP_CharacterTest.BP_CharacterTest_C|GetMaxEnergy _asbp_character_test)))))

(event EventBeginPlay)

(event Collision|EventActorBeginOverlap
  (params (OtherActor :type Actor%20Object%20Reference)))

(event EventTick
  (params (DeltaSeconds :type Float%20%28single-precision%29)))

(fn ConstructionScript)
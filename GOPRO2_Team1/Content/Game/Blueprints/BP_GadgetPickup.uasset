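; BP_GadgetPickup is a pickup for a named gadget, either Grapple or Boots, that vanishes when touched.
; Any begin overlap on its Box component destroys the actor first, with no check on what overlapped.
; It then matches GadgetName, prints it and sets GrappleGrabbed or BootsGrabbed.
; Those flags are set on the pickup itself after the destroy call, and nothing here passes them to the overlapping actor.
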(event OnComponentBeginOverlap(Box)
  (params (OverlappedComponent :type Primitive%20Component%20Object%20Reference) (OtherActor :type Actor%20Object%20Reference) (OtherComp :type Primitive%20Component%20Object%20Reference) (OtherBodyIndex :type Integer) (bFromSweep :type Boolean) (SweepResult :type Hit%20Result%20Structure%20%28by%20ref%29))
  (bind _gadgetname (Variables|Default|GetGadgetName))
  (bind _gadgetname_2 (Variables|Default|GetGadgetName))
  (Actor|DestroyActor)
  (if (Utilities|Enum|Equal(Enum) _gadgetname_2 "Grapple")
    (Development|PrintString _gadgetname_2)
    (Variables|Default|SetGrappleGrabbed true)
    (elif (Utilities|Enum|Equal(Enum) _gadgetname "Boots")
      (Development|PrintString _gadgetname)
      (Variables|Default|SetBootsGrabbed true))))

(event OnComponentEndOverlap(Box)
  (params (OverlappedComponent :type Primitive%20Component%20Object%20Reference) (OtherActor :type Actor%20Object%20Reference) (OtherComp :type Primitive%20Component%20Object%20Reference) (OtherBodyIndex :type Integer)))

(event EventBeginPlay)

(event Collision|EventActorBeginOverlap
  (params (OtherActor :type Actor%20Object%20Reference)))

(event EventTick
  (params (DeltaSeconds :type Float%20%28single-precision%29)))

(fn ConstructionScript)
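; BP_BreakingPlatform is an obstacle platform that becomes solid when BP_PaperPlayer approaches and stops being solid shortly after contact.
; It starts hidden without collision; overlapping Box enables mesh collision and arms the Box1 trigger.
; Overlapping Box1 waits a short delay, then disables mesh collision, leaving Box1 active.
; Every visibility call hides the mesh, so these graphs never show it.
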(event OnComponentBeginOverlap(Box)
  (params (OverlappedComponent :type Primitive%20Component%20Object%20Reference) (OtherActor :type Actor%20Object%20Reference) (OtherComp :type Primitive%20Component%20Object%20Reference) (OtherBodyIndex :type Integer) (bFromSweep :type Boolean) (SweepResult :type Hit%20Result%20Structure%20%28by%20ref%29))
  (Utilities|Casting|CastToBP_PaperPlayer OtherActor)
  (Rendering|SetVisibility (Variables|Default|GetStaticMesh) false false)
  (Collision|SetCollisionEnabled (Variables|Default|GetStaticMesh) "QueryAndPhysics")
  (Collision|SetCollisionEnabled (Variables|Default|GetBox1) "QueryOnly"))

(event OnComponentBeginOverlap(Box1)
  (params (OverlappedComponent :type Primitive%20Component%20Object%20Reference) (OtherActor :type Actor%20Object%20Reference) (OtherComp :type Primitive%20Component%20Object%20Reference) (OtherBodyIndex :type Integer) (bFromSweep :type Boolean) (SweepResult :type Hit%20Result%20Structure%20%28by%20ref%29))
  (Utilities|Casting|CastToBP_PaperPlayer OtherActor)
  (Utilities|FlowControl|Delay 1.5)
  (Rendering|SetVisibility (Variables|Default|GetStaticMesh) false false)
  (Collision|SetCollisionEnabled (Variables|Default|GetStaticMesh) "NoCollision"))

(event EventBeginPlay
  (Rendering|SetVisibility (Variables|Default|GetStaticMesh) false false)
  (Collision|SetCollisionEnabled (Variables|Default|GetStaticMesh) "NoCollision")
  (Collision|SetCollisionEnabled (Variables|Default|GetBox1) "NoCollision"))

(fn ConstructionScript)
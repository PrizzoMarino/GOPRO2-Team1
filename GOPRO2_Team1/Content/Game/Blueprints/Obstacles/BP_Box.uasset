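; BP_Box is a box obstacle that plays impact sounds when it hits tagged surfaces.
; Box hit events spawn a moveable-box cue for "Ground" or a splash cue for "Water" at the impact point.
; Each sound has its own DoOnce that resets after a one-second delay to prevent repeats.
; A WaterCheck overlap also detects "Water", but its spawn-sound call has no sound or location set.
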(event OnComponentHit(Box)
  (params (HitComponent :type Primitive%20Component%20Object%20Reference) (OtherActor :type Actor%20Object%20Reference) (OtherComp :type Primitive%20Component%20Object%20Reference) (NormalImpulse :type Vector :default "0, 0, 0") (Hit :type Hit%20Result%20Structure%20%28by%20ref%29))
  (bind _impactpoint (Collision|BreakHitResult Hit))
  (if (Actor|ActorHasTag OtherActor "Ground")
    (Utilities|FlowControl|DoOnce false :!label _label
      (:Completed
        (Audio|SpawnSoundatLocation "/Game/Game/Art/Anya/Audio/Level1/Moveable_box_Cue.Moveable_box_Cue" _impactpoint "0, 0, 0" 1.0 1.0 0.0 0 0)
        (Utilities|FlowControl|Delay 1.0)
        (goto _label Reset)))
    (elif (Actor|ActorHasTag OtherActor "Water")
      (Utilities|FlowControl|DoOnce false :!label _label_2
        (:Completed
          (Audio|SpawnSoundatLocation "/Game/Game/Art/Anya/Audio/Level1/Water_Splash_Cue.Water_Splash_Cue" _impactpoint "0, 0, 0" 1.0 1.0 0.0 0 0)
          (Utilities|FlowControl|Delay 1.0)
          (goto _label_2 Reset))))))

(event OnComponentBeginOverlap(WaterCheck)
  (params (OverlappedComponent :type Primitive%20Component%20Object%20Reference) (OtherActor :type Actor%20Object%20Reference) (OtherComp :type Primitive%20Component%20Object%20Reference) (OtherBodyIndex :type Integer) (bFromSweep :type Boolean) (SweepResult :type Hit%20Result%20Structure%20%28by%20ref%29))
  (if (Actor|ActorHasTag OtherActor "Water")
    (Audio|SpawnSoundatLocation 0 "0, 0, 0" "0, 0, 0" 1.0 1.0 0.0 0 0)))

(event EventBeginPlay)

(event Collision|EventActorBeginOverlap
  (params (OtherActor :type Actor%20Object%20Reference)))

(event EventTick
  (params (DeltaSeconds :type Float%20%28single-precision%29)))

(fn ConstructionScript)
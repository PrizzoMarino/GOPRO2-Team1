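; BP_DisappearingPlatform is an obstacle platform that temporarily vanishes after the paper player touches it.
; A Box overlap cast to BP_PaperPlayer starts a delayed sequence that hides the StaticMesh and disables its collision, then restores both after a few seconds.
; The IsTimerFinished flag gates the sequence so further overlaps are ignored until the platform has reappeared.
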(event OnComponentBeginOverlap(Box)
  (params (OverlappedComponent :type Primitive%20Component%20Object%20Reference) (OtherActor :type Actor%20Object%20Reference) (OtherComp :type Primitive%20Component%20Object%20Reference) (OtherBodyIndex :type Integer) (bFromSweep :type Boolean) (SweepResult :type Hit%20Result%20Structure%20%28by%20ref%29))
  (bind _asbp_paper_player (Utilities|Casting|CastToBP_PaperPlayer OtherActor))
  (Variables|Default|SetAs%20BP%20Paper%20Player _asbp_paper_player)
  (if (Variables|Default|GetisTimerFinished)
    (Variables|Default|SetisTimerFinished false)
    (Utilities|FlowControl|Delay 1.0)
    (Rendering|SetVisibility (Variables|Default|GetStaticMesh) false false)
    (Collision|SetCollisionEnabled (Variables|Default|GetStaticMesh) "NoCollision")
    (Utilities|FlowControl|Delay 3.0)
    (Rendering|SetVisibility (Variables|Default|GetStaticMesh) true false)
    (Collision|SetCollisionEnabled (Variables|Default|GetStaticMesh) "QueryAndPhysics")
    (Variables|Default|SetisTimerFinished true)))

(event EventBeginPlay)

(event Collision|EventActorBeginOverlap
  (params (OtherActor :type Actor%20Object%20Reference)))

(event EventTick
  (params (DeltaSeconds :type Float%20%28single-precision%29)))

(fn ConstructionScript)
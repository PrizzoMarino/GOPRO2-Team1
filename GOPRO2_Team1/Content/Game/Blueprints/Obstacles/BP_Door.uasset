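; BP_Door is an obstacle door that moves its static mesh with timeline-driven lerps between fixed relative positions.
; SwitchOn/Off uses a FlipFlop to alternately play and reverse one timeline, moving the mesh vertically along Z.
; OpenDoor and CloseDoor play and reverse a separate timeline, sliding the same mesh along X.
; Both paths set the mesh's whole relative location without sweep, so each overrides the other's axis.
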(event Custom|OpenDoor
  (bind _opentrack (Timeline|OpenDoorTimeline Play)
    (:Update
      (Transformation|SetRelativeLocation (Variables|Default|GetStaticMesh) (Math|Vector|Lerp(Vector) "200.000000,0.000000,0.000000" "-250.000000,0.000000,0.000000" _opentrack) false false))))

(event Custom|CloseDoor
  (bind _opentrack (Timeline|OpenDoorTimeline Reverse)
    (:Update
      (Transformation|SetRelativeLocation (Variables|Default|GetStaticMesh) (Math|Vector|Lerp(Vector) "200.000000,0.000000,0.000000" "-250.000000,0.000000,0.000000" _opentrack) false false))))

(event Custom|SwitchOn/Off
  (Utilities|FlowControl|FlipFlop
    (:A
      (bind _opentrack (Timeline|Timeline Play)
        (:Update
          (Transformation|SetRelativeLocation (Variables|Default|GetStaticMesh) (Math|Vector|Lerp(Vector) "0.000000,0.000000,-25.000000" "0.000000,0.000000,20.000000" _opentrack) false false))))
    (:B
      (Timeline|Timeline Reverse))))

(event EventBeginPlay)

(event Collision|EventActorBeginOverlap
  (params (OtherActor :type Actor%20Object%20Reference)))

(event EventTick
  (params (DeltaSeconds :type Float%20%28single-precision%29)))

(fn ConstructionScript)
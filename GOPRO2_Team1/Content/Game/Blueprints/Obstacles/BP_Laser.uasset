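; Networked laser obstacle that flags a BP_PaperPlayer as hit while it overlaps the beam.
; On the server, a looping timer flips LaserOn for "Flicker" type lasers and spawns a sound when switching on.
; LaserOn's RepNotify toggles beam visibility and collision.
; Authority-only overlap events set WasHit on entry and clear it on exit.
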(event OnComponentBeginOverlap(LaserCollision)
  (params (OverlappedComponent :type Primitive%20Component%20Object%20Reference) (OtherActor :type Actor%20Object%20Reference) (OtherComp :type Primitive%20Component%20Object%20Reference) (OtherBodyIndex :type Integer) (bFromSweep :type Boolean) (SweepResult :type Hit%20Result%20Structure%20%28by%20ref%29))
  (Networking|SwitchHasAuthority
    (:Authority
      (bind _asbp_paper_player (Utilities|Casting|CastToBP_PaperPlayer OtherActor))
      (bind _output_get (Variables|Default|SetAs%20BP%20Paper%20Player _asbp_paper_player))
      (Variables|/Game/Game/Blueprints/BP_PaperPlayer.BP_PaperPlayer_C|SetbWasHit _output_get true))))

(event OnComponentEndOverlap(LaserCollision)
  (params (OverlappedComponent :type Primitive%20Component%20Object%20Reference) (OtherActor :type Actor%20Object%20Reference) (OtherComp :type Primitive%20Component%20Object%20Reference) (OtherBodyIndex :type Integer))
  (Networking|SwitchHasAuthority
    (:Authority
      (bind _asbp_paper_player (Utilities|Casting|CastToBP_PaperPlayer OtherActor))
      (bind _output_get (Variables|Default|SetAs%20BP%20Paper%20Player _asbp_paper_player))
      (Variables|/Game/Game/Blueprints/BP_PaperPlayer.BP_PaperPlayer_C|SetbWasHit _output_get false))))

(event Custom|SRV_FlickerLaserON
  (if (Utilities|Enum|Equal(Enum) (Variables|Default|GetLaserType) "Flicker")
    (Utilities|FlowControl|FlipFlop
      (:A
        (Variables|Default|SetLaserOn true)
        (Utilities|FlowControl|DoOnce false :!label _label
          (:Completed
            (Audio|SpawnSoundatLocation "/Game/Game/Art/Anya/Audio/Level2/Laser__1__Cue.Laser__1__Cue" (Transformation|GetWorldLocation (Variables|Default|GetLaser)) "0, 0, 0" 1.0 1.0 0.0 0 0)
            (goto _label Reset))))
      (:B
        (Variables|Default|SetLaserOn false)))))

(event EventBeginPlay
  (Networking|SwitchHasAuthority
    (:Authority
      (Utilities|Time|SetTimerbyFunctionName 0 "SRV_FlickerLaserON" (Variables|Default|GetLaserOnCooldown) true false (Variables|Default|GetLaserOffCooldown)))))

(event EventTick
  (params (DeltaSeconds :type Float%20%28single-precision%29)))

(fn ConstructionScript)

(fn OnRepLaseron
  (if (Variables|Default|GetLaserOn)
    (Rendering|SetVisibility (Variables|Default|GetLaser) (Variables|Default|GetLaserOn) false)
    (Collision|SetCollisionEnabled (Variables|Default|GetLaserCollision) "QueryAndPhysics")
    (else
      (Rendering|SetVisibility (Variables|Default|GetLaser) (Variables|Default|GetLaserOn) false)
      (Collision|SetCollisionEnabled (Variables|Default|GetLaserCollision) "NoCollision"))))
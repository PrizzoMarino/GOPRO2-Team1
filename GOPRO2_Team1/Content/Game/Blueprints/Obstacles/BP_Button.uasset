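; BP_Button is an obstacle button that controls the BP_Door whose DoorValue matches its ButtonValue when BP_PaperPlayer overlaps its box.
; ButtonType selects the behavior: Press opens the door and leaves it open.
; Hold drives a timeline that slides the button and calls the door's SwitchOnOff each update, reversing on exit.
; Timed opens the door, then a looping one-second Delay counts down after exit before closing it.
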(event OnComponentBeginOverlap(Box)
  (params (OverlappedComponent :type Primitive%20Component%20Object%20Reference) (OtherActor :type Actor%20Object%20Reference) (OtherComp :type Primitive%20Component%20Object%20Reference) (OtherBodyIndex :type Integer) (bFromSweep :type Boolean) (SweepResult :type Hit%20Result%20Structure%20%28by%20ref%29))
  (bind _asbp_paper_player (Utilities|Casting|CastToBP_PaperPlayer OtherActor))
  (Variables|Default|SetAs%20BP%20Paper%20Player _asbp_paper_player)
  (bind _outactors (Actor|GetAllActorsOfClass "/Game/Game/Blueprints/Obstacles/BP_Door.BP_Door_C"))
  (bind _array_element (Utilities|Array|ForEachLoopwithBreak _outactors :!label _label)
    (:LoopBody
      (if (== (Variables|/Game/Game/Blueprints/Obstacles/BP_Door.BP_Door_C|GetDoorValue _array_element) (Variables|Default|GetButtonValue))
        (Variables|Default|SetDoorOrigin (Transformation|GetRelativeTransform (Variables|/Game/Game/Blueprints/Obstacles/BP_Door.BP_Door_C|GetStaticMesh _array_element)))
        (if (Utilities|Enum|Equal(Enum) (Variables|Default|GetButtonType) "Press")
          (Default|OpenDoor _array_element)
          (elif (Utilities|Enum|Equal(Enum) (Variables|Default|GetButtonType) "Hold")
            (bind _newtrack_0 (Timeline|Button%20Timeline Play)
              (:Update
                (Transformation|SetRelativeLocation (Variables|Default|GetButton) (Math|Vector|MakeVector (Math|Float|Lerp 0.0 -5e+01 _newtrack_0) 0.0 0.0) false false)
                (Default|SwitchOn/Off _array_element)
                (goto _label Break)))
            (elif (Utilities|Enum|Equal(Enum) (Variables|Default|GetButtonType) "Timed")
              (Variables|Default|SetDoorTime 3.0)
              (Default|OpenDoor _array_element))))))))

(event OnComponentEndOverlap(Box)
  (params (OverlappedComponent :type Primitive%20Component%20Object%20Reference) (OtherActor :type Actor%20Object%20Reference) (OtherComp :type Primitive%20Component%20Object%20Reference) (OtherBodyIndex :type Integer))
  (bind _asbp_paper_player (Utilities|Casting|CastToBP_PaperPlayer OtherActor))
  (Variables|Default|SetAs%20BP%20Paper%20Player _asbp_paper_player)
  (if (Utilities|Enum|Equal(Enum) (Variables|Default|GetButtonType) "Hold")
    (bind _newtrack_0 (Timeline|Button%20Timeline Reverse)
      (:Update
        (Transformation|SetRelativeLocation (Variables|Default|GetButton) (Math|Vector|MakeVector (Math|Float|Lerp 0.0 -5e+01 _newtrack_0) 0.0 0.0) false false)
        (Default|SwitchOn/Off (stale OnComponentBeginOverlap(Box) _array_element))
        (Utilities|Array|ForEachLoopwithBreak (stale OnComponentBeginOverlap(Box) _outactors)) ; enters at Break
      ))
    (elif (Utilities|Enum|Equal(Enum) (Variables|Default|GetButtonType) "Timed")
      (if (!= (Variables|Default|GetDoorTime) 0.0) :!label _label
        (Utilities|FlowControl|Delay 1.0)
        (Variables|Default|SetDoorTime (- (Variables|Default|GetDoorTime) 1.0))
        (goto _label)
        (else
          (Default|CloseDoor (stale OnComponentBeginOverlap(Box) _array_element)))))))

(event EventTick
  (params (DeltaSeconds :type Float%20%28single-precision%29)))

(fn ConstructionScript)
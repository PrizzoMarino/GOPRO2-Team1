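; Player character Blueprint for a networked 2D Paper flipbook game, with movement along world X, jumping, wall jumping and dashing.
; BeginPlay adds the Enhanced Input mapping context locally, and jumping while WallSlide is set launches the character up and away from its facing.
; Dash runs on client and server, launching along scaled horizontal velocity.
; UpdateAnimation picks the flipbook from falling state and speed.
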(event Custom|UpdateAnimation
  ;[1 1 1] Idle and walk anim
  (Sprite|SetFlipbook (Variables|Character|GetSprite) (select (AI|Components|NavMovement|IsFalling (Variables|Character|GetCharacterMovement)) "/Game/Test/FallingAnim.FallingAnim" (select (> (Math|Vector|VectorLength (Variables|/Script/Engine.MovementComponent|GetVelocity (Variables|Character|GetCharacterMovement))) 0.0) "/Game/Test/NewPaperFlipbook.NewPaperFlipbook" "/Game/Test/MovementTest.MovementTest"))))

(event Custom|SRV_Dash
  ;[1 1 1] Dash logic
  (CallFunction|Dash)
  (Networking|ForceNetUpdate))

(event Custom|CLIENT_Dash
  ;[1 1 1] Dash logic
  (CallFunction|Dash))

(event Input|EnhancedActionEvents|EnhancedInputActionIA_Dash
  (params (ActionValue :type Boolean) (ElapsedSeconds :type Float%20%28double-precision%29) (TriggeredSeconds :type Float%20%28double-precision%29) (InputAction :type Input%20Action%20Object%20Reference :default "/Game/Game/Blueprints/Inputs/IA_Dash.IA_Dash"))
  ;[1 1 1] Dash logic
  (:Started
    (CallFunction|CLIENTDash)
    (CallFunction|SRVDash)))

(event EventBeginPlay
  (bind _asplayer_controller (Utilities|Casting|CastToPlayerController (Pawn|GetController)))
  (if (Pawn|IsLocallyControlled)
    (Utilities|IsValid (PlayerController|LocalPlayerSubsystems|GetEnhancedInputLocalPlayerSubsystem _asplayer_controller)
      (:Is%20Valid
        (Input|AddMappingContext (PlayerController|LocalPlayerSubsystems|GetEnhancedInputLocalPlayerSubsystem _asplayer_controller) "/Game/Game/Blueprints/Inputs/IMC_Player.IMC_Player" 0 "(bIgnoreAllPressedKeysUntilRelease=True,bForceImmediately=False,bNotifyUserSettings=False)")
        (Utilities|FlowControl|Delay 0.3))
      (:Is%20Not%20Valid
        (Development|PrintString "boo")))))

(event Input|ActionEvents|InputActionJump
  (params (Key :type Key%20Structure :default "None"))
  (:Pressed
    (if (Variables|Default|GetWallSlide)
      (Character|LaunchCharacter (+ (* (Transformation|GetActorForwardVector) -6e+02) "0.000000,0.000000,800.000000") true false)
      (else
        (Character|Jump))))
  (:Released
    (Character|StopJumping)))

(event Input|AxisEvents|InputAxisMove
  (params (AxisValue :type Float%20%28single-precision%29))
  ;[1 1 1] Movement
  (Pawn|Input|AddMovementInput "1.000000,0.000000,0.000000" AxisValue false))

(fn ConstructionScript)

(fn OnRepIsDashing)

(fn Dash
  (bind _returnvalue (Transformation|GetVelocity))
  (bind _returnvalue_2 (* _returnvalue 1e+01))
  (if (not (Variables|Default|GetisDashing))
    (Variables|Default|SetisDashing true)
    (Character|LaunchCharacter (Math|Vector|MakeVector (.x _returnvalue_2) (.y _returnvalue_2) 0.0) true false)
    (Variables|Default|SetisDashing false)))
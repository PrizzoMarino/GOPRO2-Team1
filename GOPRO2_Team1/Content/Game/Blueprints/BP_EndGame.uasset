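; BP_EndGame is a trigger that starts the ending once two BP_PaperPlayer characters are inside its Box at the same time.
; Box overlap events add and remove players in an OverlappingActors array and refresh PlayerCount from its length.
; When the count reaches exactly two on entry, it calls CreateLastStoryboard on player 0's BP_MyPlayerController.
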(event OnComponentBeginOverlap(Box)
  (params (OverlappedComponent :type Primitive%20Component%20Object%20Reference) (OtherActor :type Actor%20Object%20Reference) (OtherComp :type Primitive%20Component%20Object%20Reference) (OtherBodyIndex :type Integer) (bFromSweep :type Boolean) (SweepResult :type Hit%20Result%20Structure%20%28by%20ref%29))
  (bind _overlappingactors (Variables|Default|GetOverlappingActors))
  (bind _asbp_paper_player (Utilities|Casting|CastToBP_PaperPlayer OtherActor))
  (Utilities|Set|Add _overlappingactors _asbp_paper_player)
  (bind _output_get (Variables|Default|SetPlayerCount (Utilities|Set|Length _overlappingactors)))
  (if (== _output_get 2)
    (bind _asbp_my_player_controller (Utilities|Casting|CastToBP_MyPlayerController (Game|GetPlayerController 0)))
    (Default|CreateLastStoryboard _asbp_my_player_controller)))

(event OnComponentEndOverlap(Box)
  (params (OverlappedComponent :type Primitive%20Component%20Object%20Reference) (OtherActor :type Actor%20Object%20Reference) (OtherComp :type Primitive%20Component%20Object%20Reference) (OtherBodyIndex :type Integer))
  (bind _overlappingactors (Variables|Default|GetOverlappingActors))
  (bind _asbp_paper_player (Utilities|Casting|CastToBP_PaperPlayer OtherActor))
  (Utilities|Set|Remove _overlappingactors _asbp_paper_player)
  (Variables|Default|SetPlayerCount (Utilities|Set|Length _overlappingactors)))

(fn ConstructionScript)
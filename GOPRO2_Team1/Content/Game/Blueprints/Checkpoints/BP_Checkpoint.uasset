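; BP_Checkpoint is a checkpoint actor that records its own location as the player's current checkpoint when a BP_PaperPlayer overlaps its Box.
; The location is written on every such overlap.
; For a locally controlled player, if the Checkpoint flag is set, a DoOnce plays a 2D cue and adds a checkpoint widget to the viewport a single time.
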(event OnComponentBeginOverlap(Box)
  (params (OverlappedComponent :type Primitive%20Component%20Object%20Reference) (OtherActor :type Actor%20Object%20Reference) (OtherComp :type Primitive%20Component%20Object%20Reference) (OtherBodyIndex :type Integer) (bFromSweep :type Boolean) (SweepResult :type Hit%20Result%20Structure%20%28by%20ref%29))
  (bind _asbp_paper_player (Utilities|Casting|CastToBP_PaperPlayer OtherActor))
  (bind _output_get (Variables|Default|SetAs%20BP%20Paper%20Player _asbp_paper_player))
  (bind _output_get_2 (Variables|Default|SetCheckpointLocation (Transformation|GetActorLocation)))
  (Variables|/Game/Game/Blueprints/BP_PaperPlayer.BP_PaperPlayer_C|SetCurrentCheckpoint _output_get _output_get_2)
  (if (Pawn|IsLocallyControlled _output_get)
    (if (Variables|Default|GetCheckpoint?)
      (Utilities|FlowControl|DoOnce false
        (:Completed
          (Audio|PlaySound2D "/Game/Game/Art/Anya/Audio/Level1/Checkpoint2_Cue.Checkpoint2_Cue" 1.0 1.0 0.0 0 0)
          (bind _returnvalue (UserInterface|CreateWidget "/Game/Game/Art/Anya/UI/WB_Checkpoint.WB_Checkpoint_C" (Game|GetPlayerController 0)))
          (UserInterface|Viewport|AddtoViewport _returnvalue 0))))))

(event EventBeginPlay)

(event Collision|EventActorBeginOverlap
  (params (OtherActor :type Actor%20Object%20Reference)))

(event EventTick
  (params (DeltaSeconds :type Float%20%28single-precision%29)))

(fn ConstructionScript)
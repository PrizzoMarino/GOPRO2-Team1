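; Player controller that runs the intro storyboard for each local player and hands off to gameplay in the side-scroller.
; On BeginPlay it shows WBP_FirstStoryBoard, and any key press advances its pages using the widget's progress flags.
; Server_ImDoneWithStory registers the player as ready with GM_SideScroller.
; Client_StartGameplay fades out and removes the storyboard, then enables input.
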(event Custom|Server_ImDoneWithStory
  (bind _asgm_side_scroller (Utilities|Casting|CastToGM_SideScroller (Game|GetGameMode)))
  (Default|RegisterPlayerReady _asgm_side_scroller))

(event Custom|Client_StartGameplay
  (bind _wbp_firststoryboard (Variables|Default|GetWBP_FirstStoryBoard))
  (Components|Animation|PlayAnimation _wbp_firststoryboard (Variables|/Game/Game/HUD/WBP_FirstStoryBoard.WBP_FirstStoryBoard_C|GetFadeOutBackground _wbp_firststoryboard) 0.0
    (:Finished
      (Widget|RemovefromParent (Variables|Default|GetWBP_FirstStoryBoard))
      (Input|EnableInput 0))))

(event EventTick
  (params (DeltaSeconds :type Float%20%28single-precision%29)))

(event EventBeginPlay
  (if (Pawn|IsLocalController)
    (bind _returnvalue (UserInterface|CreateWidget "/Game/Game/HUD/WBP_FirstStoryBoard.WBP_FirstStoryBoard_C"))
    (bind _output_get (Variables|Default|SetWBP_FirstStoryBoard _returnvalue))
    (UserInterface|Viewport|AddtoViewport _output_get 0)))

(event Input|KeyboardEvents|AnyKey
  (params (Key :type Key%20Structure :default "None"))
  (bind _wbp_firststoryboard (Variables|Default|GetWBP_FirstStoryBoard))
  (:Pressed
    (if (Pawn|IsLocalController)
      (if (Variables|/Game/Game/HUD/WBP_FirstStoryBoard.WBP_FirstStoryBoard_C|GetFirstFinished (Variables|Default|GetWBP_FirstStoryBoard))
        (if (Variables|/Game/Game/HUD/WBP_FirstStoryBoard.WBP_FirstStoryBoard_C|GetSecondShowing (Variables|Default|GetWBP_FirstStoryBoard))
          (if (not (Variables|/Game/Game/HUD/WBP_FirstStoryBoard.WBP_FirstStoryBoard_C|GetSecondFinished _wbp_firststoryboard))
            (if (not (Variables|/Game/Game/HUD/WBP_FirstStoryBoard.WBP_FirstStoryBoard_C|GetLastGoing (Variables|Default|GetWBP_FirstStoryBoard)))
              (Default|ChangeStoryBoardSecond _wbp_firststoryboard)))
          (elif (not (Variables|/Game/Game/HUD/WBP_FirstStoryBoard.WBP_FirstStoryBoard_C|GetSecondGoing (Variables|Default|GetWBP_FirstStoryBoard)))
            (Default|ChangeStoryBoardFirst _wbp_firststoryboard)))))))

(fn ConstructionScript)
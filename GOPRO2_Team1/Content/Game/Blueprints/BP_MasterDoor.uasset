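; BP_MasterDoor is a door actor, likely a base for variants, that slides its mesh between closed and open positions.
; BeginPlay caches the closed location and adds OpenVector to get the open one.
; OpenDoor plays a timeline that lerps the location and sets a fixed rotation, while CloseDoor reverses it; both play 2D sound, with a fallback only on opening.
; SequenceFailed is empty, and a button-location sound is unwired.
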(event EventSequenceFailed)

(event EventOpenDoor
  (if (Variables|Default|GetSound?)
    (Audio|PlaySound2D (Variables|Default|GetSound) 1.0 1.0 0.0 0 0)
    (bind _opendoor (Timeline|Timeline Play)
      (:Update
        (Transformation|SetRelativeLocationAndRotation (Variables|Default|GetDoorMesh) (Math|Vector|Lerp(Vector) (Variables|Default|GetClosedLocation) (Variables|Default|GetOpenedLocation) _opendoor) (Variables|Default|GetRotationVector) false false)))
    (else
      (Audio|PlaySound2D (Variables|Default|GetUpwardBlocks) 1.0 1.0 0.0 0 0)
      (Timeline|Timeline Play))))

(event EventCloseDoor
  (Audio|PlaySound2D (Variables|Default|GetSound) 1.0 1.0 0.0 0 0)
  (bind _opendoor (Timeline|Timeline Reverse)
    (:Update
      (Transformation|SetRelativeLocationAndRotation (Variables|Default|GetDoorMesh) (Math|Vector|Lerp(Vector) (Variables|Default|GetClosedLocation) (Variables|Default|GetOpenedLocation) _opendoor) (Variables|Default|GetRotationVector) false false))))

(event EventBeginPlay
  (bind _output_get (Variables|Default|SetClosedLocation (Variables|/Script/Engine.SceneComponent|GetRelativeLocation (Variables|Default|GetDoorMesh))))
  (Variables|Default|SetOpenedLocation (+ _output_get (Variables|Default|GetOpenVector))))

(fn ConstructionScript)
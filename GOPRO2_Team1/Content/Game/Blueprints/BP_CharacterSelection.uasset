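; BP_CharacterSelection is a walk-in character selection area that also starts the level.
; Overlapping either character box swaps the BP_PaperPlayer's skeletal mesh to a short or tall rat asset.
; The change-level box tracks overlapping players in an array with an empty OnRep, printing the count on entry.
; When the count reaches two on entry, the arriving player calls TravelToLevel1 with Map1.
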(event OnComponentBeginOverlap(BoxChar1)
  (params (OverlappedComponent :type Primitive%20Component%20Object%20Reference) (OtherActor :type Actor%20Object%20Reference) (OtherComp :type Primitive%20Component%20Object%20Reference) (OtherBodyIndex :type Integer) (bFromSweep :type Boolean) (SweepResult :type Hit%20Result%20Structure%20%28by%20ref%29))
  (bind _asbp_paper_player (Utilities|Casting|CastToBP_PaperPlayer OtherActor))
  (Components|SkeletalMesh|SetSkeletalMeshAsset (Variables|/Game/Game/Blueprints/BP_PaperPlayer.BP_PaperPlayer_C|GetSkeletalMesh _asbp_paper_player) "/Game/Game/Art/Polina/Animation/ShortRat_Anim_FallCycle.ShortRat_Anim_FallCycle"))

(event OnComponentBeginOverlap(BoxChar2)
  (params (OverlappedComponent :type Primitive%20Component%20Object%20Reference) (OtherActor :type Actor%20Object%20Reference) (OtherComp :type Primitive%20Component%20Object%20Reference) (OtherBodyIndex :type Integer) (bFromSweep :type Boolean) (SweepResult :type Hit%20Result%20Structure%20%28by%20ref%29))
  (bind _asbp_paper_player (Utilities|Casting|CastToBP_PaperPlayer OtherActor))
  (Components|SkeletalMesh|SetSkeletalMeshAsset (Variables|/Game/Game/Blueprints/BP_PaperPlayer.BP_PaperPlayer_C|GetSkeletalMesh _asbp_paper_player) "/Game/Game/Art/Polina/Animation/TallRat_Anim_idle.TallRat_Anim_idle"))

(event OnComponentBeginOverlap(BoxChangeLevel)
  (params (OverlappedComponent :type Primitive%20Component%20Object%20Reference) (OtherActor :type Actor%20Object%20Reference) (OtherComp :type Primitive%20Component%20Object%20Reference) (OtherBodyIndex :type Integer) (bFromSweep :type Boolean) (SweepResult :type Hit%20Result%20Structure%20%28by%20ref%29))
  (bind _overlappingactors (Variables|Default|GetOverlappingActors))
  (bind _asbp_paper_player (Utilities|Casting|CastToBP_PaperPlayer OtherActor))
  (Utilities|Set|Add _overlappingactors _asbp_paper_player)
  (bind _output_get (Variables|Default|SetPlayerCount (Utilities|Set|Length _overlappingactors)))
  (Development|PrintString (Utilities|String|ToString(Integer) _output_get))
  (if (== _output_get 2)
    (Default|TraveltoLevel1 _asbp_paper_player "Map1")))

(event OnComponentEndOverlap(BoxChangeLevel)
  (params (OverlappedComponent :type Primitive%20Component%20Object%20Reference) (OtherActor :type Actor%20Object%20Reference) (OtherComp :type Primitive%20Component%20Object%20Reference) (OtherBodyIndex :type Integer))
  (bind _overlappingactors (Variables|Default|GetOverlappingActors))
  (bind _asbp_paper_player (Utilities|Casting|CastToBP_PaperPlayer OtherActor))
  (Utilities|Set|Remove _overlappingactors _asbp_paper_player)
  (Variables|Default|SetPlayerCount (Utilities|Set|Length _overlappingactors)))

(fn ConstructionScript)

(fn OnRepOverlappingActors)
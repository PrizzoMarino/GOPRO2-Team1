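; Grappling hook projectile that latches onto actors tagged GrappleTarget when its sphere overlaps them.
; On a valid hit, the authority stops the projectile, sets the owning BP_PaperPlayer to flying and grappling, records the hook location and calls the player's latch confirmation.
; Overlapping anything untagged destroys the owner's current hook, without an authority check.
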(event OnComponentBeginOverlap(Sphere)
  (params (OverlappedComponent :type Primitive%20Component%20Object%20Reference) (OtherActor :type Actor%20Object%20Reference) (OtherComp :type Primitive%20Component%20Object%20Reference) (OtherBodyIndex :type Integer) (bFromSweep :type Boolean) (SweepResult :type Hit%20Result%20Structure%20%28by%20ref%29))
  (bind _returnvalue (Transformation|GetActorLocation))
  (if (Actor|ActorHasTag OtherActor "GrappleTarget")
    (Networking|SwitchHasAuthority
      (:Authority
        (Components|Movement|StopMovementImmediately (Variables|Default|GetProjectileMovement))
        (bind _asbp_paper_player (Utilities|Casting|CastToBP_PaperPlayer (Components|GetOwner)))
        (Pawn|Components|CharacterMovement|SetMovementMode (Variables|/Script/Engine.Character|GetCharacterMovement _asbp_paper_player) "MOVE_Flying" 0)
        (Variables|/Game/Game/Blueprints/BP_PaperPlayer.BP_PaperPlayer_C|SetbIsGrappling _asbp_paper_player true)
        (Variables|/Game/Game/Blueprints/BP_PaperPlayer.BP_PaperPlayer_C|SetbGrappleHitSurface _asbp_paper_player true)
        (Variables|Default|SetHookLocation (Math|Vector|MakeVector (.x _returnvalue) (.y _returnvalue) (.z _returnvalue)))
        (Transformation|AttachComponentToComponent OverlappedComponent "None" "KeepWorld" "KeepWorld" "KeepRelative" true)
        (Default|SRVConfirmHookLatched _asbp_paper_player)))
    (else
      (bind _asbp_paper_player_2 (Utilities|Casting|CastToBP_PaperPlayer (Components|GetOwner)))
      (Utilities|IsValid (Variables|/Game/Game/Blueprints/BP_PaperPlayer.BP_PaperPlayer_C|GetCurrentHook _asbp_paper_player_2)
        (:Is%20Valid
          (Actor|DestroyActor (Variables|/Game/Game/Blueprints/BP_PaperPlayer.BP_PaperPlayer_C|GetCurrentHook _asbp_paper_player_2)))))))

(event EventBeginPlay)

(event Collision|EventActorBeginOverlap
  (params (OtherActor :type Actor%20Object%20Reference)))

(event EventTick
  (params (DeltaSeconds :type Float%20%28single-precision%29)))

(fn ConstructionScript)
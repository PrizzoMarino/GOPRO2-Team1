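; BP_BreakingBlock is a cement block that breaks apart after a two-stage overlap trigger.
; Box starts with collision disabled and is armed the first time something overlaps Box1.
; The first overlap of Box waits briefly, destroys the static mesh, then enables physics and gravity on Block.
; A radial impulse at Block's location scatters it, and the actor applies heavy damage to itself.
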(event OnComponentBeginOverlap(Box)
  (params (OverlappedComponent :type Primitive%20Component%20Object%20Reference) (OtherActor :type Actor%20Object%20Reference) (OtherComp :type Primitive%20Component%20Object%20Reference) (OtherBodyIndex :type Integer) (bFromSweep :type Boolean) (SweepResult :type Hit%20Result%20Structure%20%28by%20ref%29))
  (bind _self self)
  (bind _block (Variables|Default|GetBlock))
  (Utilities|FlowControl|DoOnce false
    (:Completed
      (Utilities|FlowControl|Delay 1.5)
      (Components|DestroyComponent (Variables|Default|GetStaticMesh))
      (Physics|SetSimulatePhysics _block true)
      (Physics|SetEnableGravity (Variables|Default|GetBlock) true)
      (Physics|AddRadialImpulse _block (Transformation|GetWorldLocation (Variables|Default|GetBlock)) 5e+02 1.1e+04 "RIF_Constant" false)
      (Game|Damage|ApplyDamage _self 1e+04 (Game|GetPlayerController 0) _self))))

(event OnComponentBeginOverlap(Box1)
  (params (OverlappedComponent :type Primitive%20Component%20Object%20Reference) (OtherActor :type Actor%20Object%20Reference) (OtherComp :type Primitive%20Component%20Object%20Reference) (OtherBodyIndex :type Integer) (bFromSweep :type Boolean) (SweepResult :type Hit%20Result%20Structure%20%28by%20ref%29))
  (Utilities|FlowControl|DoOnce false
    (:Completed
      (Collision|SetCollisionEnabled (Variables|Default|GetBox) "QueryAndPhysics"))))

(event EventBeginPlay
  (Collision|SetCollisionEnabled (Variables|Default|GetBox) "NoCollision"))

(fn ConstructionScript)